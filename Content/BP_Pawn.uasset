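; Player pawn that runs a grid-based Snake game, spawning the snake and food and steering by directional input.
; Each Tick it moves the head, the start of a NextBody linked list, and appends a tail segment after food is eaten.
; Leaving the board or overlapping non-food reloads the level.
; SpawnFood replaces food using random cells and trace checks, but re-rolls the position when spawning.
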(event `self.ReceiveBeginPlay`
  (bind _returnvalue (`|SpawnActorFromClass` "/Game/BP_Head.BP_Head_C" (`KismetMathLibrary.MakeTransform` (0.0 0.0 0.0)) "Undefined" "OverrideRootScale" null null))
  (set `self.Head` _returnvalue)
  (bind _returnvalue_2 (`|SpawnActorFromClass` "/Game/BP_Body.BP_Body_C" (`KismetMathLibrary.MakeTransform` (0.0 0.0 0.0)) "Undefined" "OverrideRootScale" null null))
  (bind _output_get (set `self.End` _returnvalue_2))
  (set `/Game/BP_Snaker.NextBody` _output_get (`self.Head`))
  (add `self.OnActorBeginOverlap` (`self.Head`) (delegate `HeadOverlap`))
  (`self.SpawnFood`)
  (set `PlayerController.bShowMouseCursor` true (`GameplayStatics.GetPlayerController` 0)))

(event `HeadOverlap` :!signature `self.OnActorBeginOverlap`
  (params (OverlappedActor :type "Actor Object Reference") (OtherActor :type "Actor Object Reference"))
  (if (== (`GameplayStatics.GetObjectClass` OtherActor) "/Game/BP_Food.BP_Food_C")
    (set `self.IsEatFood` true)
    (`self.SpawnFood`)
    (`KismetSystemLibrary.PrintString` "Eat Food")
    (else
      (`self.GameOver`))))

(event `self.ReceiveTick`
  (params (DeltaSeconds :type "Float (single-precision)"))
  (bind _end (`self.End`))
  (bind _x (.x (`self.K2_GetActorLocation` (`self.Head`))))
  (bind _y (.y (`self.K2_GetActorLocation` (`self.Head`))))
  (if (or (> _x 900.0) (< _x 0.0) (> _y 900.0) (< _y 0.0))
    (`self.GameOver`)
    (else
      (`/Game/BP_Snaker.Move` (`self.Head`) (`self.SnakeLocationOffset`))
      (if (`self.IsEatFood`)
        (set `self.IsEatFood` false)
        (bind _returnvalue (`|SpawnActorFromClass` "/Game/BP_Body.BP_Body_C" (`KismetMathLibrary.MakeTransform` (- (`self.K2_GetActorLocation` _end) (`/Game/BP_Snaker.LastLocationOffset` _end))) "Undefined" "OverrideRootScale" null null))
        (bind _output_get (set `/Game/BP_Snaker.NextBody` _returnvalue (`self.End`)))
        (set `self.End` _output_get)))))

(event `InputAction|MoveUp`
  (params (Key :type "Key Structure"))
  (:`Pressed`
    (set `self.SnakeLocationOffset` (100.0 0.0 0.0))))

(event `InputAction|MoveDown`
  (params (Key :type "Key Structure"))
  (:`Pressed`
    (set `self.SnakeLocationOffset` (-100.0 0.0 0.0))))

(event `InputAction|MoveLeft`
  (params (Key :type "Key Structure"))
  (:`Pressed`
    (set `self.SnakeLocationOffset` (0.0 -100.0 0.0))))

(event `InputAction|MoveRight`
  (params (Key :type "Key Structure"))
  (:`Pressed`
    (set `self.SnakeLocationOffset` (0.0 100.0 0.0))))

(fn `GameOver`
  (`KismetSystemLibrary.PrintString` "GameOver")
  (`self.Reset`))

(fn `Reset`
  (`GameplayStatics.OpenLevel` "RetroSnaker"))

(fn `SpawnFood`
  (bind _returnvalue (`KismetMathLibrary.MakeVector` (* (`KismetMathLibrary.RandomIntegerInRange` 0 9) 100.0) (* (`KismetMathLibrary.RandomIntegerInRange` 0 9) 100.0) 150.0))
  (bind _outactors (`GameplayStatics.GetAllActorsOfClass` "/Game/BP_Food.BP_Food_C"))
  (for _array_element _outactors
    (`self.K2_DestroyActor` _array_element))
  (while (stale _returnvalue_2)
    (bind (_outhit _returnvalue_2) (`KismetSystemLibrary.LineTraceSingle` _returnvalue (- _returnvalue (0.0 0.0 100.0)) "TraceTypeQuery1")))
  (`|SpawnActorFromClass` "/Game/BP_Food.BP_Food_C" (`KismetMathLibrary.MakeTransform` (- _returnvalue (0.0 0.0 150.0))) "Undefined" "OverrideRootScale" null null))

(fn `UserConstructionScript`)